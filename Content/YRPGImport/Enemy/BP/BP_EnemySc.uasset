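; BP_EnemySc is an enemy pawn that chases the Ganyu player and takes sword damage.
; PawnSensing sight starts AIMoveTo toward the player.
; Capsule overlap with BP_祭礼剑 subtracts player AttackPower from EnemyHealth; health is checked before subtracting, so death and the player's kill-count increment come on a later hit.
; Blackboard-based patrol switching, noise response and player targeting remain as disconnected nodes, leaving their events empty.
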(event `self.ReceiveActorBeginOverlap`
  (params (OtherActor :type "Actor Object Reference"))
  ;[1 1 1] 到达目标点切换目标点
)

(event `self.ReceiveBeginPlay`)

(event `self.PawnSensing.OnSeePawn`
  (params (Pawn :type "Pawn Object Reference"))
  ;[1 1 1] 追击玩家
  (bind _asbp_ganyu_player_character (cast `/Game/ThirdPerson/Blueprints/BP_GanyuPlayerCharacter` Pawn))
  (`|AIMoveTo` self (0.0 0.0 0.0) _asbp_ganyu_player_character))

(event `self.PawnSensing.OnHearNoise`
  (params (Instigator :type "Pawn Object Reference") (Location :type "Vector Structure (by ref)") (Volume :type "Float (single-precision)"))
  ;[1 1 1] 听见噪声
)

(event `self.CapsuleComponent.OnComponentBeginOverlap`
  (params (OverlappedComponent :type "PrimitiveComponent Object Reference") (OtherActor :type "Actor Object Reference") (OtherComp :type "PrimitiveComponent Object Reference") (OtherBodyIndex :type Integer) (bFromSweep :type Boolean) (SweepResult :type "HitResult Structure (by ref)"))
  ;[1 1 1] 敌人受击
  (bind `_asbp_祭礼剑` (cast `/Game/YRPGImport/Weapon/祭礼剑/BP_祭礼剑` OtherActor))
  (`/Engine/EditorBlueprintResources/StandardMacros.IsValid` `_asbp_祭礼剑`
    (:`Is Valid`
      (if (<= (`self.EnemyHealth`) 0)
        ;[1 1 1] 击杀数量加1
        (bind _asbp_ganyu_player_character (cast `/Game/ThirdPerson/Blueprints/BP_GanyuPlayerCharacter` (`GameplayStatics.GetPlayerCharacter` 0)))
        (`/Game/ThirdPerson/Blueprints/BP_GanyuPlayerCharacter.EnemyCountAdd` _asbp_ganyu_player_character)
        (`self.K2_DestroyActor`)
        (else
          (bind _asbp_ganyu_player_character_2 (cast `/Game/ThirdPerson/Blueprints/BP_GanyuPlayerCharacter` (`GameplayStatics.GetPlayerCharacter` 0)))
          (set `self.EnemyHealth` (- (`self.EnemyHealth`) (`/Game/ThirdPerson/Blueprints/BP_GanyuPlayerCharacter.AttackPower` _asbp_ganyu_player_character_2))))))))

(fn `UserConstructionScript`)