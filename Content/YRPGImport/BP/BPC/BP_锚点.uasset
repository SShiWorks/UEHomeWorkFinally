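; Grapple anchor point actor that makes itself available to a character's hook component (AC_钩索) and shows targeting feedback.
; Sphere overlaps add or remove the anchor on the overlapping actor's hook component.
; A timeline pulses the two anchor meshes from BeginPlay, while Tick turns the Scene toward the player camera.
; Target set and cancel events animate the outer ring's scale, with setting also spawning attached Niagara effects on every timeline update.
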(event `self.Sphere.OnComponentBeginOverlap`
  (params (OverlappedComponent :type "PrimitiveComponent Object Reference") (OtherActor :type "Actor Object Reference") (OtherComp :type "PrimitiveComponent Object Reference") (OtherBodyIndex :type Integer) (bFromSweep :type Boolean) (SweepResult :type "HitResult Structure (by ref)"))
  (bind _returnvalue (`self.GetComponentByClass` OtherActor "/Game/YRPGImport/BP/BPC/AC_钩索.AC_钩索_C"))
  ;[1 1 1] 进出入锚点范围
  (`/Engine/EditorBlueprintResources/StandardMacros.IsValid` _returnvalue
    (:`Is Valid`
      (`/Game/YRPGImport/BP/BPC/AC_钩索.添加到组件` _returnvalue self))))

(event `self.Sphere.OnComponentEndOverlap`
  (params (OverlappedComponent :type "PrimitiveComponent Object Reference") (OtherActor :type "Actor Object Reference") (OtherComp :type "PrimitiveComponent Object Reference") (OtherBodyIndex :type Integer))
  (bind _returnvalue (`self.GetComponentByClass` OtherActor "/Game/YRPGImport/BP/BPC/AC_钩索.AC_钩索_C"))
  ;[1 1 1] 进出入锚点范围
  (`/Engine/EditorBlueprintResources/StandardMacros.IsValid` _returnvalue
    (:`Is Valid`
      (`/Game/YRPGImport/BP/BPC/AC_钩索.从组件移除` _returnvalue self))))

(event `self.ReceiveBeginPlay`
  ;[1 1 1] 初始化
  (`SceneComponent.SetRelativeScale3D` (`self.OutSide`) (1.0 1.0 1.0))
  (bind (_direction `_新建轨道_0`) (`Timeline|锁定呼吸效果时间轴`)
    (:`Update`
      (`SceneComponent.SetRelativeScale3D` (`self.SM_锚点_2`) (`KismetMathLibrary.Conv_DoubleToVector` (`KismetMathLibrary.Lerp` 1.0 0.63 `_新建轨道_0`)))
      (`SceneComponent.SetRelativeScale3D` (`self.SM_锚点_1`) (`KismetMathLibrary.Conv_DoubleToVector` (`KismetMathLibrary.Lerp` 1.0 0.78 `_新建轨道_0`))))))

(event `设定为目标锚点`
  ;[1 1 1] 设定为目标时的特效
  (bind (_direction `_新建轨道_0`) (`Timeline|外圈缩放时间轴` :!via `PlayFromStart`)
    (:`Update`
      (`SceneComponent.SetRelativeScale3D` (`self.OutSide`) (`KismetMathLibrary.Conv_DoubleToVector` `_新建轨道_0`))
      (bind _returnvalue (`NiagaraFunctionLibrary.SpawnSystemAttached` "/Game/YRPGImport/BP/BPC/Niagara/NS_Fx_Interact03.NS_Fx_Interact03" (`self.Scene`) "None" (0.0 0.0 0.0) (struct) "KeepRelativeOffset"))
      (`NiagaraFunctionLibrary.SpawnSystemAttached` "/Game/YRPGImport/BP/BPC/Niagara/NS_Fx_Interact05.NS_Fx_Interact05" _returnvalue "None" (0.0 0.0 0.0) (struct) "KeepRelativeOffset"))))

(event `self.ReceiveTick`
  (params (DeltaSeconds :type "Float (single-precision)"))
  ;[1 1 1] 保持正对角色
  (`SceneComponent.K2_SetWorldRotation` (`self.Scene`) (`KismetMathLibrary.FindRelativeLookAtRotation` (`self.GetTransform`) (`self.K2_GetActorLocation` (`GameplayStatics.GetPlayerCameraManager` 0))) false false))

(event `取消设定为目标锚点`
  ;[1 1 1] 取消为目标时
  (bind (_direction `_新建轨道_0`) (`Timeline|时间轴` :!via `ReverseFromEnd`)
    (:`Update`
      (`SceneComponent.SetRelativeScale3D` (`self.OutSide`) (`KismetMathLibrary.Conv_DoubleToVector` `_新建轨道_0`))
      (`KismetSystemLibrary.Delay` 0.33)
      (`SceneComponent.SetRelativeScale3D` (`self.OutSide`) (1.0 1.0 1.0)))))

(fn `UserConstructionScript`)