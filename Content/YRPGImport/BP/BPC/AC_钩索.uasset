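; Actor component that gives a player character a grappling hook, pulling it to a targeted anchor point when T is pressed.
; Each tick it picks, from a registered anchor array, the anchor best aligned with controller forward by dot product, and updates target marking.
; Firing yaws the character toward the anchor and moves it just above over a distance/speed duration, with a montage and Niagara effect.
; After that delay it zeroes velocity and stops the montage.
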(event `self.ReceiveBeginPlay`
  ;[1 1 1] 初始化
  (bind `_as角色` (cast `Character` (`self.GetOwner`)))
  (set `self.As角色` `_as角色`)
  (bind `_as玩家控制器` (cast `PlayerController` (`Pawn.GetController` `_as角色`)))
  (set `self.As玩家控制器` `_as玩家控制器`))

(event `self.ReceiveTick`
  (params (DeltaSeconds :type "Float (single-precision)"))
  (bind `_当前锚点` (`self.当前锚点`))
  ;[1 1 1] 锚点检测
  (bind _output_get (`self.锚点检测`))
  (if (not (== _output_get (`self.当前锚点`)))
    (`/Engine/EditorBlueprintResources/StandardMacros.IsValid` `_当前锚点`
      (:`Is Valid`
        (`/Game/YRPGImport/BP/BPC/BP_锚点.取消设定为目标锚点` `_当前锚点`))
      (:`Is Not Valid`
        _))
    (bind _output_get_2 (set `self.当前锚点` _output_get))
    (`/Engine/EditorBlueprintResources/StandardMacros.IsValid` _output_get_2
      (:`Is Valid`
        (`/Game/YRPGImport/BP/BPC/BP_锚点.设定为目标锚点` _output_get_2)))))

(event `CharacterRotation`
  (bind (_returnvalue_roll _returnvalue_pitch _returnvalue_yaw) (`KismetMathLibrary.BreakRotator` (`KismetMathLibrary.FindLookAtRotation` (`Actor.K2_GetActorLocation` (`self.As角色`)) (`Actor.K2_GetActorLocation` (`self.当前锚点`)))))
  ;[1 1 1] 钩索移动
  ;;[1 1 1] 位移前转向
  (`Actor.K2_SetActorRotation` (`self.As角色`) (`KismetMathLibrary.MakeRotator` 0.0 0.0 _returnvalue_yaw) false))

(event `添加到组件`
  (params (NewItem :type "/Game/YRPGImport/BP/BPC/BP_锚点 Object Reference (by ref)"))
  ;[1 1 1] 钩索移动
  ;;[1 1 1] 锚点数组管理
  (`KismetArrayLibrary.Array_Add` (`self.锚点数组`) NewItem))

(event `从组件移除`
  (params (Item :type "/Game/YRPGImport/BP/BPC/BP_锚点 Object Reference (by ref)"))
  ;[1 1 1] 钩索移动
  ;;[1 1 1] 锚点数组管理
  (`KismetArrayLibrary.Array_RemoveItem` (`self.锚点数组`) Item))

(event `CharacterMove`
  (bind `_当前锚点` (`self.当前锚点`))
  (bind `_as角色` (`self.As角色`))
  (bind (_returnvalue_x _returnvalue_y _returnvalue_z) (`KismetMathLibrary.BreakVector` (`Actor.K2_GetActorLocation` `_当前锚点`)))
  (bind _returnvalue (/ (`KismetMathLibrary.Vector_Distance` (`Actor.K2_GetActorLocation` (`self.As角色`)) (`Actor.K2_GetActorLocation` `_当前锚点`)) (`self.钩索移动速度`)))
  ;[1 1 1] 钩索移动
  ;;[1 1 1] 角色移动
  (`|ExecutionSequence`
    (:`then_0`
      (`KismetSystemLibrary.MoveComponentTo` (`Actor.RootComponent` `_as角色`) (`KismetMathLibrary.MakeVector` _returnvalue_x _returnvalue_y (+ _returnvalue_z 120.0)) (`Actor.K2_GetActorRotation` `_as角色`) false false _returnvalue))
    (:`then_1`
      (`KismetSystemLibrary.Delay` _returnvalue)
      (set `MovementComponent.Velocity` (0.0 0.0 0.0) (`Character.CharacterMovement` (`self.As角色`)))
      (`Character.StopAnimMontage` (`self.As角色`) "/Game/Characters/Ganyu/IK/Anim4钩索/GanyuStanding1HMagicAttack014UE4_Montage1.GanyuStanding1HMagicAttack014UE4_Montage1"))))

(event `Key|T`
  (params (Key :type "Key Structure"))
  (bind `_as角色` (`self.As角色`))
  ;[1 1 1] 钩索移动
  ;;[1 1 1] 按T触发
  (:`Pressed`
    (`/Engine/EditorBlueprintResources/StandardMacros.IsValid` (`self.当前锚点`)
      (:`Is Valid`
        (`self. CharacterRotation`)
        (`self.CharacterMove`)
        (`Character.PlayAnimMontage` `_as角色` "/Game/Characters/Ganyu/IK/Anim4钩索/GanyuStanding1HMagicAttack014UE4_Montage1.GanyuStanding1HMagicAttack014UE4_Montage1" 1.0 "None")
        (bind _returnvalue (`NiagaraFunctionLibrary.SpawnSystemAttached` "/Game/YRPGImport/BP/BPC/VFX/NewNiagaraSystem.NewNiagaraSystem" (`Character.Mesh` `_as角色`) "zHandTwist_R" (0.0 0.0 0.0) (struct) "KeepRelativeOffset"))
        (`NiagaraComponent.SetVariableVec3` _returnvalue "Enda" (`Actor.K2_GetActorLocation` (`self.当前锚点`)))
        (`NiagaraComponent.SetVariableFloat` _returnvalue "LifeTime" (/ (`KismetMathLibrary.Vector_Distance` (`Actor.K2_GetActorLocation` (`self.As角色`)) (`Actor.K2_GetActorLocation` (`self.当前锚点`))) (`self.钩索移动速度`)))))))

(fn `角度判断`
  (params (`钩索Actor` :type "/Game/YRPGImport/BP/BPC/BP_锚点 Object Reference"))
  (returns (ReturnValue :type "Float (double-precision)"))
  (return (`KismetMathLibrary.Dot_VectorVector` (`Actor.GetActorForwardVector` (`self.As玩家控制器`)) (`KismetMathLibrary.GetDirectionUnitVector` (`Actor.K2_GetActorLocation` (`self.As角色`)) (`Actor.K2_GetActorLocation` `钩索Actor`)))))

(fn `锚点检测`
  (returns (Output_Get :type "/Game/YRPGImport/BP/BPC/BP_锚点 Object Reference"))
  (locals (`和锚点的夹角` :type "Float (double-precision)") (`目标锚点` :type "/Game/YRPGImport/BP/BPC/BP_锚点 Object Reference"))
  (`/Engine/EditorBlueprintResources/StandardMacros.DoOnce` false :!label _label
    (:`Completed`
      (set `local.和锚点的夹角` 0.0)
      (set `local.目标锚点` null)
      (for _array_element (`self.锚点数组`)
        (bind _returnvalue (`self.角度判断` _array_element))
        (if (> _returnvalue (`local.和锚点的夹角`))
          (set `local.和锚点的夹角` _returnvalue)
          (set `local.目标锚点` _array_element)))
      (`|ExecutionSequence`
        (:`then_0`
          (return (`local.目标锚点`)))
        (:`then_1`
          (goto _label :!via `Reset`))))))