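; Character component for a Keqing-style E skill: places a marker, then teleports the owning character to it.
; First E press spawns BP_KeQinE along a camera-direction line trace; while held, a looping timer re-aims it using a fixed range instead of the 可瞬移距离 variable.
; Releasing E stops aiming.
; The next press teleports there, destroys the marker, and briefly plays an attack montage in Flying mode before restoring Walking.
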(event `self.ReceiveBeginPlay`
  ;[1 1 1] 初始化
  (bind `_as角色` (cast `Character` (`self.GetOwner`)))
  (set `self.As角色` `_as角色`)
  (bind `_as玩家控制器` (cast `PlayerController` (`Pawn.GetController` `_as角色`)))
  (set `self.As玩家控制器` `_as玩家控制器`))

(event `Key|E`
  (params (Key :type "Key Structure"))
  (bind `_e的球` (`self.E的球`))
  (bind `_as角色` (`self.As角色`))
  (bind _returnvalue (`Actor.K2_GetActorLocation` (`self.As角色`)))
  (bind _charactermovement (`Character.CharacterMovement` `_as角色`))
  ;[1 1 1] 发射生成目标
  (:`Pressed`
    (if (`self.是否有球`)
      ;[1 1 1] 瞬移到目标点
      (`Actor.K2_SetActorLocation` (`self.As角色`) (`Actor.K2_GetActorLocation` `_e的球`) false false)
      (`Actor.K2_DestroyActor` `_e的球`)
      (set `self.E的球` null)
      (set `self.是否有球` false)
      (`CharacterMovementComponent.SetMovementMode` _charactermovement "MOVE_Flying" 0)
      (`Character.PlayAnimMontage` `_as角色` "/Game/Characters/Ganyu/IK/Anim2/Sequence/02_Attack/03_Combo_Attack_03/GanyuAnim_Combo_Attack_03_02_Seq_Montage.GanyuAnim_Combo_Attack_03_02_Seq_Montage" 1.0 "None")
      (`KismetSystemLibrary.Delay` 0.5)
      (`Character.StopAnimMontage` `_as角色` "/Game/Characters/Ganyu/IK/Anim2/Sequence/02_Attack/03_Combo_Attack_03/GanyuAnim_Combo_Attack_03_02_Seq_Montage.GanyuAnim_Combo_Attack_03_02_Seq_Montage")
      (`CharacterMovementComponent.SetMovementMode` _charactermovement "MOVE_Walking" 0)
      (else
        (set `self.是否有球` true)
        (bind (_outhit _returnvalue_2) (`KismetSystemLibrary.LineTraceSingle` _returnvalue (+ _returnvalue (* (`Actor.GetActorForwardVector` (`PlayerController.PlayerCameraManager` (`self.As玩家控制器`))) (`self.可瞬移距离`))) "TraceTypeQuery1"))
        (if _returnvalue_2
          (bind (_bblockinghit _binitialoverlap _time _distance _location _impactpoint _normal _impactnormal _physmat _hitactor _hitcomponent _hitbonename _bonename _hititem _elementindex _faceindex _tracestart _traceend) (`GameplayStatics.BreakHitResult` _outhit))
          (bind _returnvalue_3 (`|SpawnActorFromClass` "/Game/YRPGImport/BP/KeQinE/BP_KeQinE.BP_KeQinE_C" (`KismetMathLibrary.MakeTransform` _location) "Undefined" "MultiplyWithRoot" null null))
          (set `self.E的球` _returnvalue_3)
          (else
            (bind _returnvalue_4 (`|SpawnActorFromClass` "/Game/YRPGImport/BP/KeQinE/BP_KeQinE.BP_KeQinE_C" (`KismetMathLibrary.MakeTransform` _traceend) "Undefined" "MultiplyWithRoot" null null))
            (set `self.E的球` _returnvalue_4)))
        (bind _returnvalue_5 (`KismetSystemLibrary.K2_SetTimerDelegate` (delegate `SettingEPosition`) 0.1 true))
        (set `self.E位置的定时器` _returnvalue_5))))
  (:`Released`
    (`KismetSystemLibrary.K2_ClearAndInvalidateTimerHandle` (`self.E位置的定时器`))))

(event `SettingEPosition`
  (bind `_e的球` (`self.E的球`))
  (bind _returnvalue (`Actor.K2_GetActorLocation` (`self.As角色`)))
  ;[1 1 1] 设定目标点位置
  (bind (_outhit _returnvalue_2) (`KismetSystemLibrary.LineTraceSingle` _returnvalue (+ _returnvalue (* (`Actor.GetActorForwardVector` (`PlayerController.PlayerCameraManager` (`self.As玩家控制器`))) 500.0)) "TraceTypeQuery1"))
  (if _returnvalue_2
    (bind (_bblockinghit _binitialoverlap _time _distance _location _impactpoint _normal _impactnormal _physmat _hitactor _hitcomponent _hitbonename _bonename _hititem _elementindex _faceindex _tracestart _traceend) (`GameplayStatics.BreakHitResult` _outhit))
    (`Actor.K2_SetActorLocation` `_e的球` _location false false)
    (else
      (`Actor.K2_SetActorLocation` `_e的球` _traceend false false))))