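; BP_KeQinE is an animated, camera-facing indicator actor with a rotating icon and two rings, apparently for KeQin's E skill.
; On BeginPlay, timelines spin the icon's yaw and drive the first ring's scale and "Max" material parameter.
; After a one-second delay, the second ring becomes visible and animates the same way on its own timeline.
; Tick rotates Root toward the player camera, billboarding the whole effect.
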(event `self.ReceiveBeginPlay`
  (bind `_圆环` (`self.圆环`))
  (bind `_圆环1` (`self.圆环1`))
  ;[1 1 1] 界面动态效果
  (`|ExecutionSequence`
    (:`then_0`
      (bind (_direction `_新建轨道_0`) (`Timeline|时间轴` :!via `PlayFromStart`)
        (:`Update`
          (`SceneComponent.K2_SetRelativeRotation` (`self.旋转图标`) (`KismetMathLibrary.MakeRotator` 0.0 0.0 `_新建轨道_0`) false false))))
    (:`then_1`
      (bind (_direction_2 `_新建轨道_0_2` `_新建轨道_1`) (`Timeline|时间轴_0` :!via `PlayFromStart`)
        (:`Update`
          (`SceneComponent.SetRelativeScale3D` `_圆环` (`KismetMathLibrary.Conv_DoubleToVector` `_新建轨道_0_2`))
          (`MeshComponent.SetScalarParameterValueOnMaterials` `_圆环` "Max" `_新建轨道_1`))))
    (:`then_2`
      (`KismetSystemLibrary.Delay` 1.0)
      (`SceneComponent.SetVisibility` (`self.圆环1`) true false)
      (bind (_direction_3 `_新建轨道_0_3` `_新建轨道_1_2`) (`Timeline|时间轴_1` :!via `PlayFromStart`)
        (:`Update`
          (`SceneComponent.SetRelativeScale3D` `_圆环1` (`KismetMathLibrary.Conv_DoubleToVector` `_新建轨道_0_3`))
          (`MeshComponent.SetScalarParameterValueOnMaterials` `_圆环1` "Max" `_新建轨道_1_2`))))))

(event `self.ReceiveTick`
  (params (DeltaSeconds :type "Float (single-precision)"))
  ;[1 1 1] 设置始终朝向玩家
  (`SceneComponent.K2_SetWorldRotation` (`self.Root`) (`KismetMathLibrary.FindLookAtRotation` (`self.K2_GetActorLocation`) (`self.K2_GetActorLocation` (`GameplayStatics.GetPlayerCameraManager` 0))) false false))

(fn `UserConstructionScript`)