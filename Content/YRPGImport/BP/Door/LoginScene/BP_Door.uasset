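; BP_Door is a double door that the player opens and closes with F while near it.
; Box overlap by a Character enables input, opens a Gate and sets the swing sign from the character's relative look-at yaw.
; A FlipFlop plays or reverses the OpenDoor timeline, which lerps both leaves to opposite yaw angles.
; Leaving the box disables input and re-triggers the FlipFlop to shut an open door.
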(event `Key|F`
  (params (Key :type "Key Structure"))
  (bind _iisdoorfrand (`self.iIsDoorFrand`))
  (:`Pressed`
    (`/Engine/EditorBlueprintResources/StandardMacros.Gate` (stale `Key|F` _isa) :!label _label
      (:`Exit`
        (bind _isa (`/Engine/EditorBlueprintResources/StandardMacros.FlipFlop` :!label _label_2)
          (:`A`
            (bind (_direction `_新建轨道_0`) (`Timeline|OpenDoor` :!label _label_3)
              (:`Update`
                (`SceneComponent.K2_SetRelativeRotation` (`self.SM_右门`) (`KismetMathLibrary.MakeRotator` 0.0 0.0 (* (`KismetMathLibrary.Lerp` 0.0 90.0 `_新建轨道_0`) _iisdoorfrand)) false false)
                (`SceneComponent.K2_SetRelativeRotation` (`self.SM_左门`) (`KismetMathLibrary.MakeRotator` 0.0 0.0 (* (`KismetMathLibrary.Lerp` 0.0 -90.0 `_新建轨道_0`) _iisdoorfrand)) false false))))
          (:`B`
            (goto _label_3 :!via `ReverseFromEnd`)))))))

(event `self.Box.OnComponentBeginOverlap`
  (params (OverlappedComponent :type "PrimitiveComponent Object Reference") (OtherActor :type "Actor Object Reference") (OtherComp :type "PrimitiveComponent Object Reference") (OtherBodyIndex :type Integer) (bFromSweep :type Boolean) (SweepResult :type "HitResult Structure (by ref)"))
  (bind `_as角色` (cast `Character` OtherActor))
  (bind (_returnvalue_roll _returnvalue_pitch _returnvalue_yaw) (`KismetMathLibrary.BreakRotator` (`KismetMathLibrary.FindRelativeLookAtRotation` (`self.GetTransform`) (`self.K2_GetActorLocation` `_as角色`))))
  (if (> _returnvalue_yaw 0.0)
    (set `self.iIsDoorFrand` 1)
    (else
      (set `self.iIsDoorFrand` -1)))
  (`self.EnableInput` (`GameplayStatics.GetPlayerController` 0))
  (goto _label :!via `Open`))

(event `self.Box.OnComponentEndOverlap`
  (params (OverlappedComponent :type "PrimitiveComponent Object Reference") (OtherActor :type "Actor Object Reference") (OtherComp :type "PrimitiveComponent Object Reference") (OtherBodyIndex :type Integer))
  (cast `Character` OtherActor)
  (`self.DisableInput` (`GameplayStatics.GetPlayerController` 0))
  (if (stale `Key|F` _isa)
    (goto _label_2)))

(fn `UserConstructionScript`)