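; Scythe weapon Blueprint that animates the weapon materializing and dissolving through material effects.
; BeginPlay creates an M_Wuqi dynamic instance for every Wuqi material slot and stores them in an array.
; 武器生成 (spawn) resets dissolve parameters, then starts three timelines driving reveal position, overall glow and pattern glow.
; 武器消散 (dissolve) drives the dissolve mask from a timeline, activating the NSWuqiXiaosan effect on each update.
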(event `self.ReceiveBeginPlay`
  (bind _wuqi (`self.wuqi`))
  (for _index (range (+ (`PrimitiveComponent.GetNumMaterials` _wuqi) 1))
    (bind _returnvalue (`PrimitiveComponent.CreateDynamicMaterialInstance` _wuqi _index "/Game/YRPGImport/Weapon/镰刀/M_Wuqi.M_Wuqi" "None"))
    (`KismetArrayLibrary.Array_Add` (`self.武器材质_0`) _returnvalue)))

(event `武器消散`
  ;[1 1 1] 注释
  (bind (_direction `_新建轨道_0`) (`Timeline|武器消散遮罩时间轴` :!via `PlayFromStart`)
    (:`Update`
      (`MaterialInstanceDynamic.SetScalarParameterValue` (`self.武器材质_0`) "消散遮罩" `_新建轨道_0`)
      (`ActorComponent.Activate` (`self.NS_WuqiXiaosan`) false))))

(event `武器生成`
  (bind `_武器材质_0` (`self.武器材质_0`))
  (`|ExecutionSequence`
    (:`then_0`
      (`MaterialInstanceDynamic.SetScalarParameterValue` (`self.武器材质_0`) "消散遮罩" 0.0)
      (`MaterialInstanceDynamic.SetScalarParameterValue` `_武器材质_0` "消散位置" 0.0))
    (:`then_1`
      (bind (_direction `_新建轨道_0`) (`Timeline|生成遮罩时间轴` :!via `PlayFromStart`)
        (:`Update`
          (`MaterialInstanceDynamic.SetScalarParameterValue` `_武器材质_0` "消散位置" `_新建轨道_0`))))
    (:`then_2`
      (bind (_direction_2 `_新建轨道_0_2`) (`Timeline|整体光亮时间轴` :!via `PlayFromStart`)
        (:`Update`
          (`MaterialInstanceDynamic.SetScalarParameterValue` (`self.武器材质_0`) "整体光强" `_新建轨道_0_2`))))
    (:`then_3`
      (bind (_direction_3 `_新建轨道_0_3`) (`Timeline|花纹光亮时间轴` :!via `PlayFromStart`)
        (:`Update`
          (`MaterialInstanceDynamic.SetScalarParameterValue` (`self.武器材质_0`) "花纹光亮" `_新建轨道_0_3`))))))

(fn `UserConstructionScript`)