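; Sacrificial Sword (祭礼剑) weapon actor that animates its appearance and dissolve through a dynamic material created on BeginPlay.
; 武器生成 (spawn) clears the dissolve mask, then starts three timelines driving the spawn mask, overall glow and pattern glow parameters.
; 武器消散 (dissolve) spawns a Niagara effect at the weapon's transform and starts the dissolve-mask timeline, whose update also activates Niagara and destroys the actor.
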(event `self.ReceiveBeginPlay`
  (bind _returnvalue (`PrimitiveComponent.CreateDynamicMaterialInstance` (`self.weapon`) 0 null "None"))
  (set `self.武器材质` _returnvalue))

(event `武器生成`
  (`|ExecutionSequence`
    (:`then_0`
      (`MaterialInstanceDynamic.SetScalarParameterValue` (`self.武器材质`) "消散遮罩" 0.0)
      (bind (_direction `_新建轨道_0`) (`Timeline|生成遮罩时间轴` :!via `PlayFromStart`)
        (:`Update`
          (`MaterialInstanceDynamic.SetScalarParameterValue` (`self.武器材质`) "生成遮罩" `_新建轨道_0`))))
    (:`then_1`
      (bind (_direction_2 `_新建轨道_0_2`) (`Timeline|整体光亮时间轴` :!via `PlayFromStart`)
        (:`Update`
          (`MaterialInstanceDynamic.SetScalarParameterValue` (`self.武器材质`) "整体光亮" `_新建轨道_0_2`))))
    (:`then_2`
      (bind (_direction_3 `_新建轨道_0_3`) (`Timeline|花纹光亮时间轴` :!via `PlayFromStart`)
        (:`Update`
          (`MaterialInstanceDynamic.SetScalarParameterValue` (`self.武器材质`) "花纹光亮" `_新建轨道_0_3`))))))

(event `武器消散`
  (bind (_returnvalue_location _returnvalue_rotation _returnvalue_scale) (`KismetMathLibrary.BreakTransform` (`SceneComponent.K2_GetComponentToWorld` (`self.weapon`))))
  (`NiagaraFunctionLibrary.SpawnSystemAtLocation` "/Game/YRPGImport/Weapon/祭礼剑/NewNiagaraSystem.NewNiagaraSystem" _returnvalue_location _returnvalue_rotation _returnvalue_scale)
  (bind (_direction `_新建轨道_0`) (`Timeline|消散遮罩时间轴` :!via `PlayFromStart`)
    (:`Update`
      (`MaterialInstanceDynamic.SetScalarParameterValue` (`self.武器材质`) "消散遮罩" `_新建轨道_0`)
      (`ActorComponent.Activate` (`self.NewNiagaraSystem`) true)
      (`self.K2_DestroyActor`))))

(fn `UserConstructionScript`)